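; GameOverFire is a fire actor for the Fire Escape game whose FireUp movement component is halted by game state or by a stopper.
; Tick polls FireEscapeGameMode's current state and zeroes FireUp's local-space velocity every frame while it is EGameOver.
; The GaveOverZone component also zeroes that velocity when it begins overlapping a Stopper actor.
; The graph neither starts the movement nor triggers game over.
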(event OnComponentBeginOverlap(GaveOverZone)
  (params (OverlappedComponent :type Primitive%20Component%20Object%20Reference) (OtherActor :type Actor%20Object%20Reference) (OtherComp :type Primitive%20Component%20Object%20Reference) (OtherBodyIndex :type Integer) (bFromSweep :type Boolean) (SweepResult :type Hit%20Result%20Structure%20%28by%20ref%29))
  (Utilities|Casting|CastToStopper OtherActor)
  (Game|Components|ProjectileMovement|SetVelocityinLocalSpace (Variables|Default|GetFireUp) "0, 0, 0"))

(event EventBeginPlay)

(event Collision|EventActorBeginOverlap
  (params (OtherActor :type Actor%20Object%20Reference)))

(event EventTick
  (params (DeltaSeconds :type Float%20%28single-precision%29))
  (if (Utilities|Select :Index (Class|FireEscapeGameMode|GetCurrentState (.AsFire%20Escape%20Game%20Mode (Utilities|Casting|CastToFireEscapeGameMode (Game|GetGameMode)))) :EPlaying false :EGameOver true :EClear false :EUnknown false)
    (Game|Components|ProjectileMovement|SetVelocityinLocalSpace (Variables|Default|GetFireUp) "0, 0, 0")))

(fn ConstructionScript)