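; Healing item pickup actor that shows a Press C prompt to the player; the heal itself is not handled here.
; While a FireEscapeCharacter overlaps HealCollision, the prompt is visible and a looping per-frame timer, used instead of Tick, yaws it toward the camera.
; Leaving hides the prompt and clears the timer.
; When GameOverFire overlaps DestroyCollision, the item spawns a steam effect and destroys itself after a short delay.
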(event OnComponentBeginOverlap(HealCollision)
  (params (OverlappedComponent :type Primitive%20Component%20Object%20Reference) (OtherActor :type Actor%20Object%20Reference) (OtherComp :type Primitive%20Component%20Object%20Reference) (OtherBodyIndex :type Integer) (bFromSweep :type Boolean) (SweepResult :type Hit%20Result%20Structure%20%28by%20ref%29))
  (Utilities|Casting|CastToFireEscapeCharacter OtherActor)
  (Rendering|SetVisibility (Variables|Default|GetPressC) true false)
  (bind _returnvalue (Utilities|Time|SetTimerbyEvent (delegate Custom|TextVector) (Utilities|Time|GetWorldDeltaSeconds) true))
  (Variables|Default|SetTimer _returnvalue))

(event OnComponentEndOverlap(HealCollision)
  (params (OverlappedComponent :type Primitive%20Component%20Object%20Reference) (OtherActor :type Actor%20Object%20Reference) (OtherComp :type Primitive%20Component%20Object%20Reference) (OtherBodyIndex :type Integer))
  (Utilities|Casting|CastToFireEscapeCharacter OtherActor)
  (Rendering|SetVisibility (Variables|Default|GetPressC) false false)
  (Utilities|Time|ClearandInvalidateTimerbyHandle (Variables|Default|GetTimer)))

(event OnComponentBeginOverlap(DestroyCollision)
  (params (OverlappedComponent :type Primitive%20Component%20Object%20Reference) (OtherActor :type Actor%20Object%20Reference) (OtherComp :type Primitive%20Component%20Object%20Reference) (OtherBodyIndex :type Integer) (bFromSweep :type Boolean) (SweepResult :type Hit%20Result%20Structure%20%28by%20ref%29))
  (Utilities|Casting|CastToGameOverFire OtherActor)
  (Effects|SpawnEmitteratLocation "/Game/StarterContent/Particles/P_Steam_Lit.P_Steam_Lit" (Transformation|GetActorLocation))
  (Utilities|FlowControl|Delay 1.0)
  (Actor|DestroyActor))

(event Custom|TextVector
  (Transformation|SetWorldRotation (Variables|Default|GetPressC) (Math|Rotator|MakeRotator 0.0 0.0 (.yaw (Math|Rotator|FindLookatRotation (Transformation|GetActorLocation) (Transformation|GetActorLocation (Game|GetPlayerCameraManager 0))))) false false))

(event EventBeginPlay)

(event Collision|EventActorBeginOverlap
  (params (OtherActor :type Actor%20Object%20Reference)))

(event EventTick
  (params (DeltaSeconds :type Float%20%28single-precision%29)))

(fn ConstructionScript)