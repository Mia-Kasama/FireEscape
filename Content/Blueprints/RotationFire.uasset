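; RotationFire is an actor that spins continuously and shatters when it meets a GameOverFire actor.
; Tick adds local roll scaled by delta time and RollPerSecond, keeping the spin frame-rate independent.
; When CylinderDestructible overlaps a GameOverFire, it applies radius damage to itself at its own location, then the actor destroys itself after a short delay.
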(event OnComponentBeginOverlap(CylinderDestructible)
  (params (OverlappedComponent :type Primitive%20Component%20Object%20Reference) (OtherActor :type Actor%20Object%20Reference) (OtherComp :type Primitive%20Component%20Object%20Reference) (OtherBodyIndex :type Integer) (bFromSweep :type Boolean) (SweepResult :type Hit%20Result%20Structure%20%28by%20ref%29))
  (bind _cylinderdestructible (Variables|Default|GetCylinderDestructible))
  (Utilities|Casting|CastToGameOverFire OtherActor)
  (Class|DestructibleComponent|ApplyRadiusDamage _cylinderdestructible 1e+02 (Transformation|GetWorldLocation _cylinderdestructible) 1e+02 1e+02 false)
  (Utilities|FlowControl|Delay 1.0)
  (Actor|DestroyActor))

(event EventBeginPlay)

(event Collision|EventActorBeginOverlap
  (params (OtherActor :type Actor%20Object%20Reference)))

(event EventTick
  (params (DeltaSeconds :type Float%20%28single-precision%29))
  (Transformation|AddActorLocalRotation (Math|Rotator|MakeRotator (* DeltaSeconds (Variables|Default|GetRollPerSecond)) 0.0 0.0) false false))

(fn ConstructionScript)