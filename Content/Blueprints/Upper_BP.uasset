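; Upper_BP is a moving destructible actor that reacts to the player, TouchTurn actors and GameOverFire actors.
; A ThirdPersonCharacter entering MoveStartCollision launches it once along SaveVector through ProjectileMovement.
; A TouchTurn actor entering MoveStopCollision zeroes its velocity.
; Overlap between MoveDestructible and GameOverFire fractures it with radius damage, then destroys the actor after a short delay.
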(event OnComponentBeginOverlap(MoveStartCollision)
  (params (OverlappedComponent :type Primitive%20Component%20Object%20Reference) (OtherActor :type Actor%20Object%20Reference) (OtherComp :type Primitive%20Component%20Object%20Reference) (OtherBodyIndex :type Integer) (bFromSweep :type Boolean) (SweepResult :type Hit%20Result%20Structure%20%28by%20ref%29))
  (Utilities|Casting|CastToThirdPersonCharacter OtherActor)
  (if true
    (Utilities|FlowControl|DoOnce false
      (:Completed
        (Game|Components|ProjectileMovement|SetVelocityinLocalSpace (Variables|Default|GetProjectileMovement) (Variables|Default|GetSaveVector))))))

(event OnComponentBeginOverlap(MoveDestructible)
  (params (OverlappedComponent :type Primitive%20Component%20Object%20Reference) (OtherActor :type Actor%20Object%20Reference) (OtherComp :type Primitive%20Component%20Object%20Reference) (OtherBodyIndex :type Integer) (bFromSweep :type Boolean) (SweepResult :type Hit%20Result%20Structure%20%28by%20ref%29))
  (bind _movedestructible (Variables|Default|GetMoveDestructible))
  (Utilities|Casting|CastToGameOverFire OtherActor)
  (Class|DestructibleComponent|ApplyRadiusDamage _movedestructible 1e+02 (Transformation|GetWorldLocation _movedestructible) 1e+02 1e+02 false)
  (Utilities|FlowControl|Delay 1.0)
  (Actor|DestroyActor))

(event OnComponentBeginOverlap(MoveStopCollision)
  (params (OverlappedComponent :type Primitive%20Component%20Object%20Reference) (OtherActor :type Actor%20Object%20Reference) (OtherComp :type Primitive%20Component%20Object%20Reference) (OtherBodyIndex :type Integer) (bFromSweep :type Boolean) (SweepResult :type Hit%20Result%20Structure%20%28by%20ref%29))
  (Utilities|Casting|CastToTouchTurn OtherActor)
  (if true
    (Game|Components|ProjectileMovement|SetVelocityinLocalSpace (Variables|Default|GetProjectileMovement) "0, 0, 0")))

(event EventBeginPlay)

(event Collision|EventActorBeginOverlap
  (params (OtherActor :type Actor%20Object%20Reference)))

(event EventTick
  (params (DeltaSeconds :type Float%20%28single-precision%29)))

(fn ConstructionScript)